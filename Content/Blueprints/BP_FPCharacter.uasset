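; BP_FPCharacter is a first-person character with camera look, replicated health and game-over handling; its movement input logic is left disconnected.
; Possession creates the HUD_InGame widget through a client event, and OnRep_CurrentHealth broadcasts health percentage changes.
; AnyDamage lowers health, while TakeDamage routes damage through BP_MainPlayerController.
; A zero-health check sets Dead and calls GameOver on every character, notifying each controller.
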(event `InputAxis|Fordwards/Backward`
  (params (AxisValue :type "Float (single-precision)"))
  ;[0.15 0.28 1 0.31] Player Movement
)

(event `InputAxis|LookUp/LookDown`
  (params (AxisValue :type "Float (single-precision)"))
  ;[0.8 0.38 0.14 0.96] Camera Rotation
  (`self.AddControllerPitchInput` (`KismetMathLibrary.FClamp` AxisValue -1.0)))

(event `InputAxis|LookRight/LookLeft`
  (params (AxisValue :type "Float (single-precision)"))
  ;[0.8 0.38 0.14 0.96] Camera Rotation
  (`self.AddControllerYawInput` (`KismetMathLibrary.FClamp` AxisValue -1.0)))

(event `InputAxis|Right/Left`
  (params (AxisValue :type "Float (single-precision)"))
  ;[0.15 0.28 1 0.31] Player Movement
)

(event `TakeDamage`
  ;[0.4 0.76 0.74 0.52] Take damage
  (bind _asbp_main_player_controller (cast `/Game/Blueprints/BP_MainPlayerController` (`self.GetController`)))
  (`/Game/Blueprints/BP_MainPlayerController.Server_Damage` _asbp_main_player_controller 1.0)
  (`self.GameOver?`))

(event `self.ReceiveAnyDamage`
  (params (Damage :type "Float (single-precision)") (DamageType :type "DamageType Object Reference") (InstigatedBy :type "Controller Object Reference") (DamageCauser :type "Actor Object Reference"))
  ;[0.19 0.5 0.96 0.15] On Any Damage Event
  (set `self.CurrentHealth` (- (`self.CurrentHealth`) Damage)))

(event `GameOver`
  ;[0.72 0.05 0.62 0.8] Game Over Screen
  (bind _asbp_main_player_controller (cast `/Game/Blueprints/BP_MainPlayerController` (`self.GetController`)))
  (`/Game/Blueprints/BP_MainPlayerController.PlayerDied` _asbp_main_player_controller (`self.Dead?`)))

(event `GameOver?`
  ;[0.72 0.05 0.62 0.8] Game Over Screen
  (if (<= (`self.CurrentHealth`) 0.0)
    (set `self.Dead?` true)
    (bind _outactors (`GameplayStatics.GetAllActorsOfClass` "BP_FPCharacter_C"))
    (`self.GameOver` _outactors)))

(event `self.ReceivePossessed`
  (params (NewController :type "Controller Object Reference"))
  ;[0.33 0.67 0.63 0.4] Create The Life Widget
  (`self.Client_CreateUI`))

(event `Client_CreateUI`
  ;[0.33 0.67 0.63 0.4] Create The Life Widget
  (bind _asbp_main_player_controller (cast `/Game/Blueprints/BP_MainPlayerController` (`self.GetController`)))
  (bind _returnvalue (`|CreateWidget` "/Game/Blueprints/HUD_Widgets/HUD_InGame.HUD_InGame_C" _asbp_main_player_controller))
  (bind _output_get (set `self.InGameWidget` _returnvalue))
  (`UserWidget.AddToViewport` _output_get 0)
  (`self.HealthChanged` (`self.GetHealthPercentage`)))

(fn `GetHealthPercentage`
  (returns (ReturnValue :type "Float (double-precision)"))
  (return (/ (`self.CurrentHealth`) (`self.MaxHealth`))))

(fn `OnRep_CurrentHealth`
  (`self.HealthChanged` (`self.GetHealthPercentage`))
  (return))

(fn `UserConstructionScript`)