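; Player controller for a turn-based, networked pistol duel with cards, creating turn, round and game-over widgets.
; While it is the player's turn, keys 1-3 shoot, shoot self or play the held card (top shot, Hanged flag, heal via negative damage).
; Shots branch to multicast or server events by authority and drive Pistola_Blueprint.
; Shots then have BP_MainGameMode cycle turns, though self-shots only when ShootSelf returns true.
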(event `Create new round`
  (bind _returnvalue (`|CreateWidget` "/Game/Blueprints/HUD_Widgets/WG_NewRound.WG_NewRound_C"))
  (bind _output_get (set `self.Widget` _returnvalue))
  (`UserWidget.AddToViewport` _output_get 0))

(event `self.ReceiveBeginPlay`
  ;[0.62 0.16 0.75 0.13] Begin Play (Show Player Turn Widget)
  (if (`self.IsLocalController`)
    (bind _returnvalue (`|CreateWidget` "/Game/Blueprints/HUD_Widgets/HUD_ShowTurn.HUD_ShowTurn_C" self))
    (`UserWidget.AddToViewport` _returnvalue 0)
    (bind _returnvalue_2 (`GameplayStatics.GetActorOfClass` "/Game/DevsTest/Luis/Pistola_Blueprint.Pistola_Blueprint_C"))
    (set `self.Pistola` _returnvalue_2)
    (`self.Create new round`)))

(event `Start Turn CLIENT`
  ;[0.25 0.68 0.47 0.29] Start And End Turn On Client
  (`self.SetMyTurn` true))

(event `Server_Damage`
  (params (BaseDamage :type "Float (single-precision)"))
  ;[0.63 0.79 0.6 0.23] Server Damage Function
  (`GameplayStatics.ApplyDamage` (`self.K2_GetPawn`) BaseDamage))

(event `PlayerDied`
  (params (`Died?` :type Boolean))
  (bind _returnvalue (`|CreateWidget` "/Game/Blueprints/HUD_Widgets/HUD_InGame.HUD_InGame_C"))
  (bind _output_get (set `self.HUD` _returnvalue))
  (`UserWidget.AddToViewport` _output_get 0)
  (`/Game/Blueprints/HUD_Widgets/HUD_InGame.Active GameOver Image` (`self.HUD`) `Died?`))

(event `End Turn CLIENT`
  ;[0.25 0.68 0.47 0.29] Start And End Turn On Client
  (`self.SetMyTurn` false))

(event `Key|One`
  (params (Key :type "Key Structure"))
  ;[0.22 0.87 0.6 0.96] Input Action Example
  (:`Pressed`
    (if (`self.MyTurn?`)
      (if (`KismetSystemLibrary.IsServer`)
        (`self.Shoot Multicast`)
        (else
          (`self.Shoot Server`))))))

(event `Shoot Multicast`
  (`self.Shoot`)
  (if (`/Game/Blueprints/BP_FPCharacter.Hanged` (`self.PlayerCharacter`))
    (set `/Game/Blueprints/BP_FPCharacter.Hanged` false (`self.PlayerCharacter`) :!label _label)))

(event `Shoot Top Multicast`
  (`self.ShootTop`))

(event `Shoot Server`
  (`self.Shoot`)
  (if (`/Game/Blueprints/BP_FPCharacter.Hanged` (`self.PlayerCharacter`))
    (goto _label)))

(event `Shoot Top Server`
  (`self.ShootTop`))

(event `Key|Two`
  (params (Key :type "Key Structure"))
  ;[0.17 0.52 0.54 0.36] Shoot self Input
  (:`Pressed`
    (if (`self.MyTurn?`)
      (if (`KismetSystemLibrary.IsServer`)
        (`self.ShootSelf Multicast`)
        (else
          (`self.ShootSelf Server`))))))

(event `ShootSelf Multicast`
  (`self.ShootSelf`)
  (if (`/Game/Blueprints/BP_FPCharacter.Hanged` (`self.PlayerCharacter`))
    (`/Game/Blueprints/BP_FPCharacter.TakeCard` (`self.PlayerCharacter`))
    (set `/Game/Blueprints/BP_FPCharacter.Hanged` false (`self.PlayerCharacter`) :!label _label_2)))

(event `ShootSelf Server`
  (`self.ShootSelf`)
  (if (`/Game/Blueprints/BP_FPCharacter.Hanged` (`self.PlayerCharacter`))
    (`/Game/Blueprints/BP_FPCharacter.TakeCard` (`self.PlayerCharacter`))
    (goto _label_2)))

(event `Key|Three`
  (params (Key :type "Key Structure"))
  (bind _playercharacter (`self.PlayerCharacter`))
  ;[0.17 0.52 0.54 0.36] Card input
  (:`Pressed`
    (if (`self.MyTurn?`)
      (switch `int` (`/Game/Blueprints/BP_FPCharacter.CardIndex` _playercharacter)
        (:`0`
          (if (`KismetSystemLibrary.IsServer`)
            (`self.Shoot Top Multicast`)
            (else
              (`self.Shoot Top Server`))))
        (:`1`
          (set `/Game/Blueprints/BP_FPCharacter.Hanged` true _playercharacter))
        (:`2`
          (`GameplayStatics.ApplyDamage` _playercharacter -1.0)))
      (set `/Game/Blueprints/BP_FPCharacter.CardIndex` 10 _playercharacter)
      (`/Game/Blueprints/HUD_Widgets/WG_NewRound.HideCard` (`self.Widget`)))))

(event `Server Action - Shoot`
  ;[0.08 0.19 0.97 0.22] Do It Action On Server And End Turn Example
  (bind _asbp_main_game_mode (cast `/Game/Blueprints/BP_MainGameMode` (`GameplayStatics.GetGameMode`)))
  (`/Game/Blueprints/BP_MainGameMode.Cycle Turns` _asbp_main_game_mode))

(event `Server Action - UseItem`)

(fn `SetMyTurn`
  (params (MyTurn :type Boolean))
  (bind _output_get (set `self.MyTurn?` MyTurn))
  (`self.OnMyTurnChanged` _output_get))

(fn `Shoot`
  (locals (NewLocalVar :type "/Game/DevsTest/Luis/Pistola_Blueprint Object Reference"))
  (bind _returnvalue (`GameplayStatics.GetActorOfClass` "/Game/DevsTest/Luis/Pistola_Blueprint.Pistola_Blueprint_C"))
  (bind _output_get (set `self.Pistola` _returnvalue))
  (`/Game/DevsTest/Luis/Pistola_Blueprint.ShootNormal` _output_get)
  (`self.Server Action - Shoot`))

(fn `ShootSelf`
  (bind _returnvalue (`GameplayStatics.GetActorOfClass` "/Game/DevsTest/Luis/Pistola_Blueprint.Pistola_Blueprint_C"))
  (bind _output_get (set `self.Pistola` _returnvalue))
  (bind _newparam (`/Game/DevsTest/Luis/Pistola_Blueprint.ShootSelf` _output_get))
  (if _newparam
    (`self.Server Action - Shoot`)))

(fn `ShootTop`
  (bind _returnvalue (`GameplayStatics.GetActorOfClass` "/Game/DevsTest/Luis/Pistola_Blueprint.Pistola_Blueprint_C"))
  (bind _output_get (set `self.Pistola` _returnvalue))
  (`/Game/DevsTest/Luis/Pistola_Blueprint.ShootTop` _output_get)
  (`self.Server Action - Shoot`))

(fn `UserConstructionScript`)